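; BP_TrainingTurret_WeakObjectPool is a training turret that spawns its bullets through the PITS weak object pool subsystem.
; On BeginPlay, after the parent's logic, it creates a pool for the bullet class at the requested size.
; Its Shoot event acquires one pooled bullet per spawn point, placed at that point's world transform, with no explicit release in this Blueprint.
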(event `self.ReceiveBeginPlay`
  (`parent.ReceiveBeginPlay`)
  ; Creates the pool
  (`PITS_WeakObjectPoolSubsystem.CreateObjectPool` (subsystem `PITS_WeakObjectPoolSubsystem`) (`self.BulletClass`) (`self.RequestedPoolSize`)))

(event `PITS_ShooterInterface.Shoot`
  ; Retrieves object from pool
  (for _array_element (`self.SpawnPoints`)
    (`PITS_WeakObjectPoolSubsystem.AcquirePooledObject` (subsystem `PITS_WeakObjectPoolSubsystem`) (`self.BulletClass`) (`SceneComponent.K2_GetComponentToWorld` _array_element))))

(fn `UserConstructionScript`)