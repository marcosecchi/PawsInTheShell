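; Training turret actor that demonstrates bullet spawning through an object pool while spinning continuously.
; On BeginPlay it gathers its arrow components as spawn points, creates a bullet pool in the PITS object pool subsystem if none exists, and starts a timeline-driven yaw rotation.
; Shoot acquires a pooled bullet at each arrow's transform.
; The looping fire-rate timer setup is disconnected, so nothing in this graph triggers shooting.
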(event `self.ReceiveBeginPlay`
  (bind _returnvalue (subsystem `PITS_ObjectPoolSubsystem`))
  (`KismetSystemLibrary.DelayUntilNextTick`)
  (`|ExecutionSequence`
    (:`then_0`
      ; Gat all arrow components to be used as spawn points.
      (set `self.SpawnPoints` (`self.K2_GetComponentsByClass` "/Script/Engine.ArrowComponent")))
    (:`then_1`
      ; Creates the pool size
      (if (not (`PITS_ObjectPoolSubsystem.HasObjectPool` _returnvalue (`self.BulletClass`)))
        (`PITS_ObjectPoolSubsystem.CreateObjectPool` _returnvalue (`self.BulletClass`) (`self.RequestedPoolSize`))))
    (:`then_3`
      ; Start rotating the turret
      (`TimelineComponent.SetPlayRate` (`self.Timeline`) (`self.RotationPlayRate`))
      (bind (_direction _alpha) (`Timeline|Timeline`)
        (:`Update`
          (`SceneComponent.K2_SetRelativeRotation` (`self.Turret`) (`KismetMathLibrary.MakeRotator` 0.0 0.0 (* _alpha 360.0)) false false))))))

(event `Shoot`
  ; Retrieves object from pool
  (for _array_element (`self.SpawnPoints`)
    (`PITS_ObjectPoolSubsystem.AcquirePooledObject` (subsystem `PITS_ObjectPoolSubsystem`) (`self.BulletClass`) (`SceneComponent.K2_GetComponentToWorld` _array_element))))

(fn `UserConstructionScript`)