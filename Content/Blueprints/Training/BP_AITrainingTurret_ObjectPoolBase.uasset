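; Base training turret actor that spawns bullets from an object pool, leaving the firing logic to subclasses.
; On BeginPlay it waits a tick, collects its arrow components as spawn points, and creates a pool for the bullet class through the PITS object pool subsystem if none exists.
; A timeline then spins the turret's yaw at a configurable play rate, while Shoot only prints a reminder to implement it.
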(event `self.ReceiveBeginPlay`
  (bind _returnvalue (subsystem `PITS_ObjectPoolSubsystem`))
  (`KismetSystemLibrary.DelayUntilNextTick`)
  (`|ExecutionSequence`
    (:`then_0`
      ; Gat all arrow components to be used as spawn points.
      (set `self.SpawnPoints` (`self.K2_GetComponentsByClass` "/Script/Engine.ArrowComponent")))
    (:`then_1`
      ; Creates the pool size
      (if (not (`PITS_ObjectPoolSubsystem.HasObjectPool` _returnvalue (`self.BulletClass`)))
        (`PITS_ObjectPoolSubsystem.CreateObjectPool` _returnvalue (`self.BulletClass`) (`self.RequestedPoolSize`))))
    (:`then_2`
      ; Start rotating the turret
      (if (> (`self.RotationPlayRate`) 0.0)
        (`TimelineComponent.SetPlayRate` (`self.Timeline`) (`self.RotationPlayRate`))
        (bind (_direction _alpha) (`Timeline|Timeline`)
          (:`Update`
            (`SceneComponent.K2_SetRelativeRotation` (`self.Turret`) (`KismetMathLibrary.MakeRotator` 0.0 0.0 (* _alpha 360.0)) false false)))))))

(event `PITS_ShooterInterface.Shoot`
  (`KismetSystemLibrary.PrintString` "Implement shoot logic from subclasses." true true (struct :`R` 1.0 :`G` 0.219967 :`A` 1.0)))

(fn `UserConstructionScript`)