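; BP_TrainingTurret_01 is a training turret that rotates and fires pooled bullets from all of its arrow components at a fixed rate.
; On BeginPlay it gathers the arrows as spawn points, creates a bullet pool in the PITS world subsystem if none exists, and starts a looping fire timer.
; Each tick of that timer acquires a pooled bullet at every arrow's world transform, while a timeline drives the turret's yaw.
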(event `self.ReceiveBeginPlay`
  (bind _returnvalue (subsystem `PITS_WorldSubsystem`))
  (`|ExecutionSequence`
    (:`then_0`
      ; Gat all arrow components to be used as spawn points.
      (set `self.SpawnPoints` (`self.K2_GetComponentsByClass` "/Script/Engine.ArrowComponent")))
    (:`then_1`
      ; Creates the pool size
      (if (not (`PITS_WorldSubsystem.HasObjectPool` _returnvalue (`self.BulletClass`)))
        (`PITS_WorldSubsystem.CreateObjectPool` _returnvalue (`self.BulletClass`) (`self.RequestedPoolSize`))))
    (:`then_2`
      ; Set timer for spawning
      (`KismetSystemLibrary.K2_SetTimerDelegate` (`|CreateDelegate` :!event `OnTimer`) (`self.FireRate`) true))
    (:`then_3`
      ; Start rotating the turret
      (`TimelineComponent.SetPlayRate` (`self.Timeline`) (`self.RotationPlayRate`))
      (bind (_direction _alpha) (`Timeline|Timeline`)
        (:`Update`
          (`SceneComponent.K2_SetRelativeRotation` (`self.Turret`) (`KismetMathLibrary.MakeRotator` 0.0 0.0 (* _alpha 360.0)) false false))))))

(event `OnTimer`
  ; Retrieves object from pool
  (for _array_element (`self.SpawnPoints`)
    (`PITS_WorldSubsystem.AcquirePooledObject` (subsystem `PITS_WorldSubsystem`) (`self.BulletClass`) (`SceneComponent.K2_GetComponentToWorld` _array_element))))

(fn `UserConstructionScript`)