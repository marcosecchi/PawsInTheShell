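; BP_TrainingTargetSpawner is a training actor that periodically places pooled targets at random spawn points in the level.
; On BeginPlay it creates a one-object pool through the PITS world subsystem, caches all spawn-point actors and starts a looping timer.
; Each timer tick requests a pooled target and, if valid, moves it to a random cached point's location without spawning new actors.
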(event `self.ReceiveBeginPlay`
  (`|ExecutionSequence`
    (:`then_0`
      ; Initialize the object pool
      (`PITS_WorldSubsystem.CreateObjectPool` (subsystem `PITS_WorldSubsystem`) (`self.SpawnableTargetClass`) 1))
    (:`then_1`
      ; Get spawn points
      (bind _outactors (`GameplayStatics.GetAllActorsOfClass` (`self.SpawnPointClass`)))
      (set `self.TargetBases` _outactors))
    (:`then_2`
      ; Start the spawn loop
      (`KismetSystemLibrary.K2_SetTimerDelegate` (`|CreateDelegate` :!event `OnTimer`) (`self.SpawnTime`) true))))

(event `OnTimer`
  ; Is there a spawn location available?
  (if (> (`KismetArrayLibrary.Array_Length` (`self.TargetBases`)) 0)
    ; Acquire an object from the pool
    (bind _returnvalue (`PITS_WorldSubsystem.GetPooledObject` (subsystem `PITS_WorldSubsystem`) (`self.SpawnableTargetClass`)))
    (if (`KismetSystemLibrary.IsValid` _returnvalue)
      ; Position the pooled object
      (`self.K2_SetActorLocation` _returnvalue (`self.K2_GetActorLocation` (`KismetArrayLibrary.Array_Random` (`self.TargetBases`))) false false))))

(fn `UserConstructionScript`)