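; AI training turret Blueprint that fires bullets from an object pool.
; On BeginPlay it runs the parent logic, then asks the PITS object pool subsystem to create a pool for its bullet class at the requested size if none exists.
; Its Shoot event acquires one pooled bullet at the world transform of each spawn point.
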(event `self.ReceiveBeginPlay`
  (bind _returnvalue (subsystem `PITS_ObjectPoolSubsystem`))
  (`parent.ReceiveBeginPlay`)
  ; Creates the pool size
  (if (not (`PITS_ObjectPoolSubsystem.HasObjectPool` _returnvalue (`self.BulletClass`)))
    (`PITS_ObjectPoolSubsystem.CreateObjectPool` _returnvalue (`self.BulletClass`) (`self.RequestedPoolSize`))))

(event `PITS_ShooterInterface.Shoot`
  ; Retrieves object from pool
  (for _array_element (`self.SpawnPoints`)
    (`PITS_ObjectPoolSubsystem.AcquirePooledObject` (subsystem `PITS_ObjectPoolSubsystem`) (`self.BulletClass`) (`SceneComponent.K2_GetComponentToWorld` _array_element))))

(fn `UserConstructionScript`)