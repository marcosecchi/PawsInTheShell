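; BP_TrainingTurretActivator selects which training turret variants remain in the level by destroying the others when play begins.
; On BeginPlay, three boolean flags each gate a pass that finds every actor of one turret class and destroys it.
; The classes cover object-pool, weak-object-pool and no-pool turrets, so each pooling approach can be removed independently.
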(event `self.ReceiveBeginPlay`
  (`|ExecutionSequence`
    (:`then_0`
      (if (`self.DestroyPooledTurrets`)
        (bind _outactors (`GameplayStatics.GetAllActorsOfClass` "/Game/Blueprints/Training/BP_TrainingTurret_ObjectPool.BP_TrainingTurret_ObjectPool_C"))
        (for _array_element _outactors
          (`self.K2_DestroyActor` _array_element))))
    (:`then_1`
      (if (`self.DestroyWeakPooledTurrets`)
        (bind _outactors_2 (`GameplayStatics.GetAllActorsOfClass` "/Game/Blueprints/Training/BP_TrainingTurret_WeakObjectPool.BP_TrainingTurret_WeakObjectPool_C"))
        (for _array_element_2 _outactors_2
          (`self.K2_DestroyActor` _array_element_2))))
    (:`then_2`
      (if (`self.DestroyNonPooledTurrets`)
        (bind _outactors_3 (`GameplayStatics.GetAllActorsOfClass` "/Game/Blueprints/Training/BP_TrainingTurret_NoObjectPool.BP_TrainingTurret_NoObjectPool_C"))
        (for _array_element_3 _outactors_3
          (`self.K2_DestroyActor` _array_element_3))))))

(fn `UserConstructionScript`)