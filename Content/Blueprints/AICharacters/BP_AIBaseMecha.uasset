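; BP_AIBaseMecha is an AI mecha character Blueprint with a separate head mesh and a widget that displays its health.
; On BeginPlay it attaches the head to the body mesh's mech_head socket and caches the user widget from its widget container.
; It then binds to health status updates, pushing the initial and each subsequent health percentage to the widget, so the UI refreshes by event.
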(event `self.ReceiveBeginPlay`
  (`|ExecutionSequence`
    (:`then_0`
      ;[1 1 1] Locks the head to the corresponding socket
      (`SceneComponent.K2_AttachToComponent` (`self.HeadMesh`) (`self.Mesh`) "mech_head" "KeepRelative" "KeepRelative" "KeepWorld" true))
    (:`then_1`
      ;[1 1 1] Saves a reference to the health widget
      (set `self.PlayerWidget` (`WidgetComponent.GetUserWidgetObject` (`self.WidgetContainer`))))
    (:`then_2`
      ;[1 1 1] Binds to health updates
      (add `PITS_BaseCharacter.OnUpdateHealthStatus` (delegate `OnHealthStatusUpdate`))
      (message `PITS_StatsWidgetInterface.UpdateHealth` (`self.PlayerWidget`) (`PITS_HealthInterface.GetHealthPercentage`)))))

(event `OnHealthStatusUpdate`
  (params (HealthPercentage :type "Float (single-precision)"))
  ;[1 1 1] Updates the UI
  (message `PITS_StatsWidgetInterface.UpdateHealth` (`self.PlayerWidget`) HealthPercentage))

(fn `UserConstructionScript`)