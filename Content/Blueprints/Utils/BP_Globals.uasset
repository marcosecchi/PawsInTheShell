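; BP_Globals is a utility Blueprint that centralizes shared color constants for health and PicoTech displays.
; Each function returns a hard-coded color: good, bad and critical health tiers, enemy health, and PicoTech idle and attack states.
; Enemy health uses the same red as critical health, though it has its own function.
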(fn `GetEnemyHealthColor`
  (returns (Result :type "LinearColor Structure"))
  (return (struct :`R` 1.0 :`B` 0.033285 :`A` 1.0)))

(fn `GetHealthColor_Bad`
  (returns (Result :type "LinearColor Structure"))
  (return (struct :`R` 1.0 :`G` 0.736654 :`A` 1.0)))

(fn `GetHealthColor_Critical`
  (returns (Result :type "LinearColor Structure"))
  (return (struct :`R` 1.0 :`B` 0.033285 :`A` 1.0)))

(fn `GetHealthColor_Good`
  (returns (Result :type "LinearColor Structure"))
  (return (struct :`G` 0.541225 :`B` 1.0 :`A` 1.0)))

(fn `GetPicoTechColor_Attack`
  (returns (Result :type "LinearColor Structure"))
  (return (struct :`R` 1.0 :`G` 0.27641 :`B` 0.265625 :`A` 1.0)))

(fn `GetPicoTechColor_Idle`
  (returns (Result :type "LinearColor Structure"))
  (return (struct :`R` 1.0 :`G` 1.0 :`B` 1.0 :`A` 1.0)))