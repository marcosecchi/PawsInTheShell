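; BP_TileBase is a base tile actor whose shape is set by a TileId describing which of its four cardinal sides are open.
; InitTile clamps the incoming ID, then Init shows it on a text render and queries HasDirection for each side.
; CheckConnection destroys the directional static mesh of every closed side, leaving only meshes for open connections, so the trimming is one-way.
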(event `/Game/Blueprints/Interfaces/WangTileInterface.InitTile`
  (params (TileId :type Integer))
  (set `self.TileId` (`KismetMathLibrary.Clamp` TileId -1 15))
  (`self.Init`))

(fn `CheckConnection`
  (params (MeshComponent :type "StaticMeshComponent Object Reference") (IsOpen :type Boolean))
  (if (not IsOpen)
    (`ActorComponent.K2_DestroyComponent` MeshComponent)
    (return)))

(fn `Init`
  (`|ExecutionSequence`
    (:`then_0`
      (`TextRenderComponent.K2_SetText` (`self.TextRender`) (`KismetTextLibrary.Conv_IntToText` (`self.TileId`))))
    (:`then_1`
      (`self.CheckConnection` (`self.StaticMesh_N`) (`MazeGeneratorFunctionLibrary.HasDirection` (`self.TileId`) "North")))
    (:`then_2`
      (`self.CheckConnection` (`self.StaticMesh_S`) (`MazeGeneratorFunctionLibrary.HasDirection` (`self.TileId`) "South")))
    (:`then_3`
      (`self.CheckConnection` (`self.StaticMesh_E`) (`MazeGeneratorFunctionLibrary.HasDirection` (`self.TileId`) "East")))
    (:`then_4`
      (`self.CheckConnection` (`self.StaticMesh_W`) (`MazeGeneratorFunctionLibrary.HasDirection` (`self.TileId`) "West")))))

(fn `UserConstructionScript`)