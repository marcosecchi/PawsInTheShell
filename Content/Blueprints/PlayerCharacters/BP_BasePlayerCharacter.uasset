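; Base player character Blueprint that sets up a police back badge and an overhead-style widget showing name and health.
; On BeginPlay it attaches the badge to the mesh's Badge socket, then caches the widget from the widget container and sends it the character name.
; A health update event forwards the percentage to the widget through interface messages, keeping the UI decoupled from the character.
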(event `self.ReceiveBeginPlay`
  (`|ExecutionSequence`
    (:`then_0`
      ;[1 1 1] Locks the Police back badge to the corresponding socket
      (`SceneComponent.K2_AttachToComponent` (`self.PoliceBadge`) (`self.Mesh`) "Badge" "KeepRelative" "KeepRelative" "KeepWorld" true))
    (:`then_1`
      ;[1 1 1] Saves a reference to the health widget
      (bind _output_get (set `self.PlayerWidget` (`WidgetComponent.GetUserWidgetObject` (`self.WidgetContainer`))))
      ;[1 1 1] Updates the player dysplay name by means of an interface
      (message `PITS_StatsWidgetInterface.UpdateName` _output_get (`self.CharacterName`)))))

(event `self.HandleUpdateHealthStatus`
  (params (HealthPercentage :type "Float (single-precision)"))
  ;[1 1 1] Updates the UI
  (message `PITS_StatsWidgetInterface.UpdateHealth` (`self.PlayerWidget`) HealthPercentage))

(fn `UserConstructionScript`)