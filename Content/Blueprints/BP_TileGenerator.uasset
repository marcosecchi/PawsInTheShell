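; BP_TileGenerator is an actor that builds a tiled maze in the level at BeginPlay.
; It calls GenerateMaze with its Data to get a Map keyed by grid coordinates, then spawns a randomly chosen class from TileClasses for each key.
; Tiles are offset from the actor's location by Spacing, with X negated, and each receives its map value through an InitTile interface message.
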(event `self.ReceiveBeginPlay`
  (bind (_returnvalue_x _returnvalue_y _returnvalue_z) (`KismetMathLibrary.BreakVector` (`self.K2_GetActorLocation`)))
  (bind _spacing (`self.Spacing`))
  (bind _returnvalue (`MazeGeneratorFunctionLibrary.GenerateMaze` (`self.Data`)))
  (bind _output_get (set `self.Map` _returnvalue))
  (bind _keys (`BlueprintMapLibrary.Map_Keys` _output_get))
  (for _array_element _keys
    (bind (_x _y) (break `IntVector` _array_element))
    (bind _returnvalue_2 (`|SpawnActorFromClass` (`KismetArrayLibrary.Array_Random` (`self.TileClasses`)) (`KismetMathLibrary.MakeTransform` (`KismetMathLibrary.MakeVector` (+ (* _x _spacing -1.0) _returnvalue_x) (+ (* _y _spacing) _returnvalue_y) _returnvalue_z)) "Undefined" "MultiplyWithRoot" null null))
    (message `/Game/Blueprints/Interfaces/WangTileInterface.InitTile` _returnvalue_2 (`BlueprintMapLibrary.Map_Find` (`self.Map`) _array_element))))

(fn `UserConstructionScript`)