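; BP_ParallelSpawner is an actor that triggers a batch spawn of actors around its own location shortly after play begins.
; After a brief delay on BeginPlay, StartSpawnParallel prints a status message and calls SpawnActorsParallel on PITSWorldSubsystem.
; It passes its class, min/max amount and radius variables with its location as center, leaving the spawning itself to the subsystem.
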(event `StartSpawnParallel`
  (`KismetSystemLibrary.PrintString` "Spawning Actors")
  (`PITS_WorldSubsystem.SpawnActorsParallel` (subsystem `PITS_WorldSubsystem`) (`self.SpawnableActorClass`) (`self.MinAmount`) (`self.MaxAmount`) (`self.K2_GetActorLocation`) (`self.SpawnRadius`)))

(event `self.ReceiveBeginPlay`
  (`KismetSystemLibrary.Delay` 1.0)
  (`self.StartSpawnParallel`))

(fn `UserConstructionScript`)