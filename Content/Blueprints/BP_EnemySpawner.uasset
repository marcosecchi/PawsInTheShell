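; Enemy spawner Blueprint that periodically spawns enemies at locations chosen by an Environment Query.
; A looping BeginPlay timer drives an EQS query run from the spawner, picking randomly from the best 25% of results.
; When the query finishes, the first result is stored as SpawnLocation and SpawnEnemy is called.
; GetSpawnTransform supplies that location with the spawner's rotation and unit scale.
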(event `self.ReceiveBeginPlay`
  (`KismetSystemLibrary.K2_SetTimerDelegate` (`|CreateDelegate` :!event `OnSpawn`) 3.0 true))

(event `OnSpawn`
  ; Find a spawn location through an Environment Query
  (bind _returnvalue (`EnvQueryManager.RunEQSQuery` (`self.Query`) self "RandomBest25Pct"))
  (add `EnvQueryInstanceBlueprintWrapper.OnQueryFinishedEvent` _returnvalue (`|CreateDelegate` :!event `OnQueryFinished`)))

(event `OnQueryFinished`
  (params (QueryInstance :type "EnvQueryInstanceBlueprintWrapper Object Reference") (QueryStatus :type "EEnvQueryStatus Enum" :default "Processing"))
  ; Store the spawn location and spawn the enemy
  (bind _resultlocations (`EnvQueryInstanceBlueprintWrapper.GetQueryResultsAsLocations` QueryInstance))
  (set `self.SpawnLocation` (`|GetArrayItem` _resultlocations))
  (`self.SpawnEnemy`))

(fn `GetSpawnTransform`
  (returns (ReturnValue :type "Transform Structure"))
  (return (`KismetMathLibrary.MakeTransform` (`self.SpawnLocation`) (`self.K2_GetActorRotation`))))

(fn `UserConstructionScript`)