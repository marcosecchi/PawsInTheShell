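; BP_DamageZone_PicoTech is a damage zone Blueprint that drives PicoTech particle visuals; its graphs contain no damage logic.
; The construction script sizes the particle effect radius and scales spawn rate from the DamageZoneVolume sphere radius.
; Actor overlap begin switches particles to the attack color and sets their attractor to the zone's own location.
; Overlap end restores the idle color, without filtering or counting overlapping actors.
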(event `self.ReceiveActorBeginOverlap`
  (params (OtherActor :type "Actor Object Reference"))
  (bind _picotechparticles (`self.PicoTechParticles`))
  (`FXSystemComponent.SetColorParameter` _picotechparticles "ParticleColor" (`/Game/Blueprints/Utils/BP_Globals.GetPicoTechColor_Attack`))
  (`FXSystemComponent.SetVectorParameter` _picotechparticles "AttractorPosition" (`self.K2_GetActorLocation`)))

(event `self.ReceiveActorEndOverlap`
  (params (OtherActor :type "Actor Object Reference"))
  (`FXSystemComponent.SetColorParameter` (`self.PicoTechParticles`) "ParticleColor" (`/Game/Blueprints/Utils/BP_Globals.GetPicoTechColor_Idle`)))

(fn `UserConstructionScript`
  (bind _picotechparticles (`self.PicoTechParticles`))
  (bind _sphereradius (`SphereComponent.SphereRadius` (`self.DamageZoneVolume`)))
  (`NiagaraComponent.SetVariableFloat` _picotechparticles "EffectRadius" _sphereradius)
  (`NiagaraComponent.SetVariableFloat` _picotechparticles "SpawnRate" (/ _sphereradius 10.0)))