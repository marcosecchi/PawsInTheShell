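; BP_TrainingTarget is a pooled training target that pops up, spins, stays for a random time, then disappears.
; A timeline started on BeginPlay drives the mesh's yaw rotation.
; On pool acquire, a pop-in timeline scales the actor, followed by a random delay within a min/max range.
; A pop-out timeline then scales it again and releases it through the PITS world subsystem on finish.
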(event `PITS_PooledObjectInterface.HandleAcquire`
  ; Handle PITS_PooledObjectInterface
  (`self.ShowTarget`))

(event `self.ReceiveBeginPlay`
  ; Handle infinite loop rotation
  (bind (_direction _alpha) (`Timeline|RotateTimeline`)
    (:`Update`
      (`SceneComponent.K2_SetRelativeRotation` (`self.StaticMesh`) (`KismetMathLibrary.MakeRotator` 0.0 0.0 (* _alpha 360.0)) false false))))

(event `ShowTarget`
  (bind (_direction _alpha) (`Timeline|PopinTimeline` :!via `PlayFromStart`)
    (:`Update`
      ; Popup scale
      (`self.SetActorScale3D` (`KismetMathLibrary.Conv_DoubleToVector` _alpha)))
    (:`Finished`
      ; Hide after a random delay
      (`KismetSystemLibrary.Delay` (`KismetMathLibrary.RandomFloatInRange` (`self.MinTimeActive`) (`self.MaxTimeActive`)))
      (`self.HideTarget`))))

(event `HideTarget`
  (bind (_direction _alpha) (`Timeline|PopoutTimeline` :!via `PlayFromStart`)
    (:`Update`
      ; Popout scale
      (`self.SetActorScale3D` (`KismetMathLibrary.Conv_DoubleToVector` _alpha)))
    (:`Finished`
      ; Releases the object from the pool
      (`PITS_WorldSubsystem.ReleasePooledObject` (subsystem `PITS_WorldSubsystem`) self))))

(fn `UserConstructionScript`)